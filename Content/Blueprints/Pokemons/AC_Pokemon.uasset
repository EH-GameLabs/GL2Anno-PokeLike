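; AC_Pokemon is a Pokemon component that serves as the entry point for attacks on an opposing Pokemon.
; OnAttackOpponent looks up a move by index in PokemonStats and passes it with the opponent to AttackOpponent.
; AttackOpponent is unfinished: it only checks that the opponent has an AC_Pokemon component and applies no effect.
; A test event fires the first move at the current opposite Pokemon.
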(event Custom|OnAttackOpponent
  (params (MoveIndex :type Integer) (Opponent%20Pkm :type BP%20Pkm%20Test%20Object%20Reference))
  (CallFunction|AttackOpponent (Utilities|Array|Get(acopy) (.PokemonMoves (Utilities|Struct|BreakPokemonStats (Variables|Pokemon|GetPokemonStats))) MoveIndex) Opponent%20Pkm))

(event Custom|TEST%20Attack
  (CallFunction|OnAttackOpponent 0 (Variables|Pokemon|GetCurrentOppositePkm)))

(fn AttackOpponent
  (params (Attack%20Move :type Pkm%20Move%20Structure) (Opponent%20Pkm :type BP%20Pkm%20Test%20Object%20Reference))
  (Utilities|IsValid (Actor|GetComponentbyClass Opponent%20Pkm "AC_Pokemon_C")))