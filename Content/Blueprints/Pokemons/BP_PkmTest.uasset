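; BP_PkmTest is a test Pokémon actor that joins the player's party when something overlaps it.
; Its BoxCollision overlap event passes the ACPokemon component's stats to GI_MonsterSystem's AddPokemonToYourTeam, prints the new party length, then destroys the actor.
; The overlapping actor is not filtered, and a disconnected branch that would grant XP to the Pokémon never runs.
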(event OnComponentBeginOverlap(BoxCollision)
  (params (OverlappedComponent :type Primitive%20Component%20Object%20Reference) (OtherActor :type Actor%20Object%20Reference) (OtherComp :type Primitive%20Component%20Object%20Reference) (OtherBodyIndex :type Integer) (bFromSweep :type Boolean) (SweepResult :type Hit%20Result%20Structure%20%28by%20ref%29))
  ;[0.15 0.15 0.15 0.5] PURO TEST
  (bind _asgi_monster_system (Utilities|Casting|CastToGI_MonsterSystem (Game|GetGameInstance)))
  (Default|AddPokemontoYourTeam _asgi_monster_system (Variables|/Game/Blueprints/Pokemons/AC_Pokemon.AC_Pokemon_C|GetPokemonStats (Variables|Default|GetAC_Pokemon)))
  (Development|PrintString (Utilities|String|Append "Added to list " "Now Length is: " (Utilities|String|ToString(Integer) (Utilities|Array|Length (Variables|/Game/ThirdPerson/Blueprints/BP_Exploration/GI_MonsterSystem.GI_MonsterSystem_C|GetPlayerPokemonParty _asgi_monster_system)))))
  (Actor|DestroyActor))

(event EventBeginPlay)

(event Collision|EventActorBeginOverlap
  (params (OtherActor :type Actor%20Object%20Reference)))

(event EventTick
  (params (DeltaSeconds :type Float%20%28single-precision%29)))

(fn ConstructionScript)