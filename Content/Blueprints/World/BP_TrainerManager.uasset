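; BP_TrainerManager keeps the defeated state of trainers in sync with the saved game.
; On BeginPlay, after a short delay, it prints the saved array's length and marks each trainer flagged in the save as defeated.
; DefeatTrainer finds a trainer by RowName and passes its array index to the game instance.
; Saved flags map to trainers purely by array index, so the Trainers order matters.
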(event Custom|DefeatTrainer
  (params (Trainer :type Name))
  (bind _array_element (Utilities|Array|ForEachLoopwithBreak (Variables|Default|GetTrainers) :!label _label)
    (:LoopBody
      (if (== (Variables|/Game/Blueprints/World/BP_TrainerNPC.BP_TrainerNPC_C|GetRowName _array_element) Trainer)
        (Variables|Default|SetArray%20Element _array_element)
        (goto _label Break)))
    (:Completed
      (Default|DefeatTrainer (CallFunction|GetPkmGameInstance) (Utilities|Array|FindItem (Variables|Default|GetTrainers) (Variables|Default|GetArray%20Element))))))

(event EventBeginPlay
  (bind _asgi_monster_system (CallFunction|GetPkmGameInstance))
  (bind _savegameref (Variables|/Game/ThirdPerson/Blueprints/BP_Exploration/GI_MonsterSystem.GI_MonsterSystem_C|GetSaveGameRef _asgi_monster_system))
  (bind _trainers (Variables|/Game/Inventory/Blueprints/BP_SaveGame.BP_SaveGame_C|GetTrainers _savegameref))
  ;[0.15 0.15 0.15 0.5] che schifo
  (Utilities|FlowControl|Delay 0.1)
  (Development|PrintString (Utilities|String|Append "Length: " (Utilities|String|ToString(Integer) (Utilities|Array|Length _trainers))))
  (for (_array_element _array_index) _trainers
    (if _array_element
      (Default|SetIsDefeated (Utilities|Array|Get(acopy) (Variables|Default|GetTrainers) _array_index)))))

(fn ConstructionScript)