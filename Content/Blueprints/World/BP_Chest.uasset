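; BP_Chest is an interactable world chest that gives the player potions, super potions, Poké Balls or Mega Balls.
; A collision sphere registers the chest as the third-person character's CurrentInteractable on overlap and clears it on exit.
; OnInteract switches on ChestType and adds Quantity of that item through the Pkm game instance.
; The graph has no opened state, so nothing here limits repeat looting.
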(event OnComponentBeginOverlap(SphereCollision)
  (params (OverlappedComponent :type Primitive%20Component%20Object%20Reference) (OtherActor :type Actor%20Object%20Reference) (OtherComp :type Primitive%20Component%20Object%20Reference) (OtherBodyIndex :type Integer) (bFromSweep :type Boolean) (SweepResult :type Hit%20Result%20Structure%20%28by%20ref%29))
  (bind _asbp_third_person_character (Utilities|Casting|CastToBP_ThirdPersonCharacter OtherActor))
  (Variables|/Game/ThirdPerson/Blueprints/BP_ThirdPersonCharacter.BP_ThirdPersonCharacter_C|SetCurrentInteractable _asbp_third_person_character self))

(event OnComponentEndOverlap(SphereCollision)
  (params (OverlappedComponent :type Primitive%20Component%20Object%20Reference) (OtherActor :type Actor%20Object%20Reference) (OtherComp :type Primitive%20Component%20Object%20Reference) (OtherBodyIndex :type Integer))
  (bind _asbp_third_person_character (Utilities|Casting|CastToBP_ThirdPersonCharacter OtherActor))
  (Variables|/Game/ThirdPerson/Blueprints/BP_ThirdPersonCharacter.BP_ThirdPersonCharacter_C|SetCurrentInteractable _asbp_third_person_character 0))

(event EventOnInteract
  (switch Utilities|FlowControl|Switch|SwitchonItemType (Variables|Chest|GetChestType)
    (:NewEnumerator0
      (Default|AddPotion (CallFunction|GetPkmGameInstance) (Variables|Chest|GetQuantity)))
    (:NewEnumerator1
      (Default|AddSuperPotion (CallFunction|GetPkmGameInstance) (Variables|Chest|GetQuantity)))
    (:NewEnumerator2
      (Default|AddPokeball (CallFunction|GetPkmGameInstance) (Variables|Chest|GetQuantity)))
    (:NewEnumerator3
      (Default|AddMegaball (CallFunction|GetPkmGameInstance) (Variables|Chest|GetQuantity)))))

(fn ConstructionScript)