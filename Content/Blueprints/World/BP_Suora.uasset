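; BP_Suora is an interactable world actor that heals the player's Pokémon for a fee.
; Its Box overlap sets or clears itself as the CurrentInteractable on BP_ThirdPersonCharacter.
; On interact, it calls HealAllPokemon on the game instance, then PayForHealing subtracts HealingPrice from the save game's money, clamped at zero.
; Healing runs without an affordability check, so it succeeds even when money is short.
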(event OnComponentBeginOverlap(Box)
  (params (OverlappedComponent :type Primitive%20Component%20Object%20Reference) (OtherActor :type Actor%20Object%20Reference) (OtherComp :type Primitive%20Component%20Object%20Reference) (OtherBodyIndex :type Integer) (bFromSweep :type Boolean) (SweepResult :type Hit%20Result%20Structure%20%28by%20ref%29))
  (bind _asbp_third_person_character (Utilities|Casting|CastToBP_ThirdPersonCharacter OtherActor))
  (Variables|/Game/ThirdPerson/Blueprints/BP_ThirdPersonCharacter.BP_ThirdPersonCharacter_C|SetCurrentInteractable _asbp_third_person_character self))

(event OnComponentEndOverlap(Box)
  (params (OverlappedComponent :type Primitive%20Component%20Object%20Reference) (OtherActor :type Actor%20Object%20Reference) (OtherComp :type Primitive%20Component%20Object%20Reference) (OtherBodyIndex :type Integer))
  (bind _asbp_third_person_character (Utilities|Casting|CastToBP_ThirdPersonCharacter OtherActor))
  (Variables|/Game/ThirdPerson/Blueprints/BP_ThirdPersonCharacter.BP_ThirdPersonCharacter_C|SetCurrentInteractable _asbp_third_person_character 0))

(event EventBeginPlay)

(event Collision|EventActorBeginOverlap
  (params (OtherActor :type Actor%20Object%20Reference)))

(event EventTick
  (params (DeltaSeconds :type Float%20%28single-precision%29)))

(event EventOnInteract
  (bind _asgi_monster_system (CallFunction|GetPkmGameInstance))
  (Default|HealAllPokemon _asgi_monster_system)
  (CallFunction|PayforHealing _asgi_monster_system))

(fn ConstructionScript)

(fn PayforHealing
  (params (self2 :type GI%20Monster%20System%20Object%20Reference))
  (bind _savegameref (Variables|/Game/ThirdPerson/Blueprints/BP_Exploration/GI_MonsterSystem.GI_MonsterSystem_C|GetSaveGameRef self2))
  (Variables|/Game/Inventory/Blueprints/BP_SaveGame.BP_SaveGame_C|SetSavedMoneyAmount _savegameref (Math|Integer|Max(Integer) (- (Variables|/Game/Inventory/Blueprints/BP_SaveGame.BP_SaveGame_C|GetSavedMoneyAmount _savegameref) (Variables|Default|GetHealingPrice)))))