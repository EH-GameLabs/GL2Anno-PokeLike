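; BP_AtmPkm is an interactable world terminal that opens the Pokémon ATM UI.
; Its box overlap sets or clears itself as the third-person character's current interactable.
; On interact, it pushes WBP_AtmPkmUI onto the world HUD's UI, initializes its Pokémon, then switches to UI-only input and shows the mouse cursor.
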(event OnComponentBeginOverlap(Box)
  (params (OverlappedComponent :type Primitive%20Component%20Object%20Reference) (OtherActor :type Actor%20Object%20Reference) (OtherComp :type Primitive%20Component%20Object%20Reference) (OtherBodyIndex :type Integer) (bFromSweep :type Boolean) (SweepResult :type Hit%20Result%20Structure%20%28by%20ref%29))
  (bind _asbp_third_person_character (Utilities|Casting|CastToBP_ThirdPersonCharacter OtherActor))
  (Variables|/Game/ThirdPerson/Blueprints/BP_ThirdPersonCharacter.BP_ThirdPersonCharacter_C|SetCurrentInteractable _asbp_third_person_character self))

(event OnComponentEndOverlap(Box)
  (params (OverlappedComponent :type Primitive%20Component%20Object%20Reference) (OtherActor :type Actor%20Object%20Reference) (OtherComp :type Primitive%20Component%20Object%20Reference) (OtherBodyIndex :type Integer))
  (bind _asbp_third_person_character (Utilities|Casting|CastToBP_ThirdPersonCharacter OtherActor))
  (Variables|/Game/ThirdPerson/Blueprints/BP_ThirdPersonCharacter.BP_ThirdPersonCharacter_C|SetCurrentInteractable _asbp_third_person_character 0))

(event EventBeginPlay)

(event Collision|EventActorBeginOverlap
  (params (OtherActor :type Actor%20Object%20Reference)))

(event EventTick
  (params (DeltaSeconds :type Float%20%28single-precision%29)))

(event EventOnInteract
  (bind _hud_world (CallFunction|GetWorldHUD))
  (bind _returnvalue (Game|GetPlayerController 0))
  (bind _worldui (Variables|/Game/Blueprints/World/HUD_World.HUD_World_C|GetWorldUI _hud_world))
  (Default|PushWorldUI _worldui "/Game/Blueprints/UI/World/WBP_AtmPkmUI.WBP_AtmPkmUI_C")
  (bind _aswbp_atm_pkm_ui (Utilities|Casting|CastToWBP_AtmPkmUI (Variables|/Game/Blueprints/UI/World/WBP_WorldUI.WBP_WorldUI_C|GetCurrentActiveWidget _worldui)))
  (Default|InitializePokemons _aswbp_atm_pkm_ui)
  (Input|SetInputModeUIOnly _returnvalue 0 "DoNotLock" false)
  (Variables|/Script/Engine.PlayerController|SetbShowMouseCursor _returnvalue true))

(fn ConstructionScript)