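; BP_TrainerNPC is an overworld trainer that challenges the player to a Pokémon-style battle when they enter its vision cone.
; The first overlap saves the player's transform, shows timed dialogue with movement frozen, then starts the battle through the game instance, using its row name and BP_TrainerManager index.
; Later overlaps only toggle player interaction.
; SetIsDefeated disables the cone's collision.
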(event OnComponentBeginOverlap(VisionCone)
  (params (OverlappedComponent :type Primitive%20Component%20Object%20Reference) (OtherActor :type Actor%20Object%20Reference) (OtherComp :type Primitive%20Component%20Object%20Reference) (OtherBodyIndex :type Integer) (bFromSweep :type Boolean) (SweepResult :type Hit%20Result%20Structure%20%28by%20ref%29))
  (bind _asbp_third_person_character (Utilities|Casting|CastToBP_ThirdPersonCharacter OtherActor))
  (if (Variables|Default|GetHasChallenged)
    (Variables|/Game/ThirdPerson/Blueprints/BP_ThirdPersonCharacter.BP_ThirdPersonCharacter_C|SetCanInteract _asbp_third_person_character true)
    (Variables|/Game/ThirdPerson/Blueprints/BP_ThirdPersonCharacter.BP_ThirdPersonCharacter_C|SetRowNameTrainer _asbp_third_person_character (Variables|Default|GetRowName))
    (else
      (Variables|Default|SetHasChallenged true)
      (Variables|/Game/ThirdPerson/Blueprints/BP_Exploration/GI_MonsterSystem.GI_MonsterSystem_C|SetPlayerPos (CallFunction|GetPkmGameInstance) (Transformation|GetActorTransform _asbp_third_person_character))
      ;[0.15 0.15 0.15 0.5] DIALOGHI
      (Components|Activation|Deactivate (Variables|/Script/Engine.Character|GetCharacterMovement _asbp_third_person_character))
      (Default|StartTrainerDialogue _asbp_third_person_character)
      (Utilities|FlowControl|Delay 3.0)
      (Default|RemoveTrainerDialogue _asbp_third_person_character)
      (Components|Activation|Activate (Variables|/Script/Engine.Character|GetCharacterMovement _asbp_third_person_character) false)
      (bind _returnvalue (Actor|GetActorOfClass "/Game/Blueprints/World/BP_TrainerManager.BP_TrainerManager_C"))
      (Default|StartTrainerBattle (CallFunction|GetPkmGameInstance) (Variables|Default|GetRowName) (Utilities|Array|FindItem (Variables|/Game/Blueprints/World/BP_TrainerManager.BP_TrainerManager_C|GetTrainers _returnvalue) self)))))

(event OnComponentEndOverlap(VisionCone)
  (params (OverlappedComponent :type Primitive%20Component%20Object%20Reference) (OtherActor :type Actor%20Object%20Reference) (OtherComp :type Primitive%20Component%20Object%20Reference) (OtherBodyIndex :type Integer))
  (bind _asbp_third_person_character (Utilities|Casting|CastToBP_ThirdPersonCharacter OtherActor))
  (if (Variables|Default|GetHasChallenged)
    (Variables|/Game/ThirdPerson/Blueprints/BP_ThirdPersonCharacter.BP_ThirdPersonCharacter_C|SetCanInteract _asbp_third_person_character false)))

(event Custom|SetIsDefeated
  (Collision|SetCollisionEnabled (Variables|Default|GetVisionCone) "NoCollision"))

(event EventBeginPlay)

(event Collision|EventActorBeginOverlap
  (params (OtherActor :type Actor%20Object%20Reference)))

(event EventTick
  (params (DeltaSeconds :type Float%20%28single-precision%29)))

(fn ConstructionScript)