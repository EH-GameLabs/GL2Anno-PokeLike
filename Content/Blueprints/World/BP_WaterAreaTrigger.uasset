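; BP_WaterAreaTrigger is a world trigger volume that can start wild monster battles when the player enters it.
; On EncounterBox overlap, a third-person character with CanFindPkm set gets one random roll against EncounterChance.
; A success saves the player's transform to the game instance, then calls StartWildBattle with the Encounters data.
; A timer-based repeat roll through TryEncounter remains in the graph but is disconnected.
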(event OnComponentBeginOverlap(EncounterBox)
  (params (OverlappedComponent :type Primitive%20Component%20Object%20Reference) (OtherActor :type Actor%20Object%20Reference) (OtherComp :type Primitive%20Component%20Object%20Reference) (OtherBodyIndex :type Integer) (bFromSweep :type Boolean) (SweepResult :type Hit%20Result%20Structure%20%28by%20ref%29))
  (bind _asbp_third_person_character (Utilities|Casting|CastToBP_ThirdPersonCharacter OtherActor))
  (if (Variables|/Game/ThirdPerson/Blueprints/BP_ThirdPersonCharacter.BP_ThirdPersonCharacter_C|GetCanFindPkm _asbp_third_person_character)
    (if (<= (Math|Random|RandomFloat) (Variables|Exploration|GetEncounterChance))
      (Development|PrintString "TRUE")
      (CallFunction|SavePlayerPos _asbp_third_person_character)
      (Default|StartWildBattle (CallFunction|GetPkmGameInstance) (Variables|Exploration|GetEncounters))
      (else
        (Development|PrintString "FALSE")))))

(event OnComponentEndOverlap(EncounterBox)
  (params (OverlappedComponent :type Primitive%20Component%20Object%20Reference) (OtherActor :type Actor%20Object%20Reference) (OtherComp :type Primitive%20Component%20Object%20Reference) (OtherBodyIndex :type Integer))
  (Utilities|Casting|CastToBP_ThirdPersonCharacter OtherActor))

(event EventBeginPlay)

(event Collision|EventActorBeginOverlap
  (params (OtherActor :type Actor%20Object%20Reference)))

(event EventTick
  (params (DeltaSeconds :type Float%20%28single-precision%29)))

(fn ConstructionScript)

(fn TryEncounter
  (if (< (Math|Random|RandomFloatinRange 0.0 1.0) (Variables|Exploration|GetEncounterChance))
    (bind _asgi_monster_system (Utilities|Casting|CastToGI_MonsterSystem (Game|GetGameInstance))
      (:then
        (Default|StartWildBattle _asgi_monster_system (Variables|Exploration|GetEncounters))
        (Utilities|Time|ClearTimerbyFunctionName 0 "TryEncounter")
        (Development|PrintText "Hello"))
      (:CastFailed
        (Development|PrintText "cast failed")))
    (else
      (Development|PrintText "false"))))

(fn SavePlayerPos
  (params (Player :type Character%20Object%20Reference))
  (Variables|/Game/ThirdPerson/Blueprints/BP_Exploration/GI_MonsterSystem.GI_MonsterSystem_C|SetPlayerPos (CallFunction|GetPkmGameInstance) (Transformation|GetActorTransform Player)))