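; BP_CollectiblesManager tracks collectible chests in the level and keeps their collected state across saves.
; On BeginPlay, after a short delay, it reads the save game's Collectibles flags and destroys each chest in its Chests array whose flag is set.
; CollectChest looks up a chest's index in that array and forwards it to the game instance, so array order ties chests to save slots.
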(event Custom|Collect%20Chest
  (params (NewParam :type BP%20Chest%20Object%20Reference))
  (Default|CollectChest (CallFunction|GetPkmGameInstance) (Utilities|Array|FindItem (Variables|Default|GetChests) NewParam)))

(event EventBeginPlay
  (bind _asgi_monster_system (CallFunction|GetPkmGameInstance))
  (bind _savegameref (Variables|/Game/ThirdPerson/Blueprints/BP_Exploration/GI_MonsterSystem.GI_MonsterSystem_C|GetSaveGameRef _asgi_monster_system))
  (bind _collectibles (Variables|/Game/Inventory/Blueprints/BP_SaveGame.BP_SaveGame_C|GetCollectibles _savegameref))
  ;[0.15 0.15 0.15 0.5] che schifo
  (Utilities|FlowControl|Delay 0.1)
  (Development|PrintString (Utilities|String|Append "Length: " (Utilities|String|ToString(Integer) (Utilities|Array|Length _collectibles))))
  (for (_array_element _array_index) _collectibles
    (if _array_element
      (Actor|DestroyActor (Utilities|Array|Get(acopy) (Variables|Default|GetChests) _array_index)))))

(fn ConstructionScript)