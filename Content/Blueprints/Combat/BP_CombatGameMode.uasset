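; Game mode running turn-based Pokémon-style battles between the player's and enemy's parties.
; It waits for the combat HUD, shows actions, then resolves moves (ordered by Agility), switches, items or fleeing, handling faints, XP and battle end.
; Damage combines an Attack/Defense power formula, Luck-based crits, random variance and a type multiplier always keyed to the player's Pokémon type.
; Party state lives in the game instance and is pushed to the UI.
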(event Custom|Enemy%20Attack
  ;[0 0 0 0.5] CUSTOM EVENTS
  (Battle|EnemyAttacking)
  (TurnManager|UpdateUI))

(event Custom|OnSelectedPkmAction
  ;[0 0 0 0.5] Resolve Actions
  (Utilities|FlowControl|Delay 1.0)
  (switch Utilities|FlowControl|Switch|SwitchonActionType (Variables|Default|GetActionType)
    (:NewEnumerator4
      (Development|PrintString "ERROR" true true "(R=1.000000,G=0.000000,B=0.000000,A=1.000000)"))
    (:NewEnumerator0
      (if (Battle|CheckFirstAttacker)
        (CallFunction|PlayerAttack)
        (if (Variables|Default|GetIsEnemyDead)
          (CallFunction|EnemyDefeated)
          (else
            (Utilities|FlowControl|Delay 1.0)
            (CallFunction|EnemyAttack)
            (if (Variables|Default|GetIsPlayerDead)
              (CallFunction|PlayerDefeated)
              (else
                (CallFunction|TurnFinished)))))
        (else
          (CallFunction|EnemyAttack)
          (if (Variables|Default|GetIsPlayerDead)
            (CallFunction|PlayerDefeated)
            (else
              (Utilities|FlowControl|Delay 1.0)
              (CallFunction|PlayerAttack)
              (if (Variables|Default|GetIsEnemyDead)
                (CallFunction|EnemyDefeated)
                (else
                  (CallFunction|TurnFinished))))))))
    (:NewEnumerator1
      ;;[0 0 0 0.5] CAMBIO -> Scelta Player
      (UIHelper|UpdatePlayerUI)
      (CallFunction|EnemyAttack)
      (if (Variables|Default|GetIsPlayerDead)
        (CallFunction|PlayerDefeated)
        (else
          (CallFunction|TurnFinished))))
    (:NewEnumerator2
      (CallFunction|EnemyAttack)
      (if (Variables|Default|GetIsPlayerDead)
        (CallFunction|PlayerDefeated)
        (else
          (CallFunction|TurnFinished))))
    (:NewEnumerator5
      ;;[0 0 0 0.5] CAMBIO -> Pokemon sconfitto
      (UIHelper|UpdatePlayerUI)
      (CallFunction|TurnFinished))
    (:NewEnumerator6
      ;;[0 0 0 0.5] FUGA
      (TurnManager|EndBattle))))

(event Custom|TurnFinished
  ;[0 0 0 0.5] CUSTOM EVENTS
  (TurnManager|EndTurn)
  (CallFunction|StartTurn))

(event Custom|Player%20Defeated
  ;[0 0 0 0.5] CUSTOM EVENTS
  (if (Default|HasPlayerPokemontoFight (CallFunction|GetPkmGameInstance))
    (Default|ShowPokemonList (Variables|/Game/Blueprints/Combat/HUD_Combat.HUD_Combat_C|GetWBP%20CombatUI (CallFunction|GetCombatHUD)))
    (else
      (Development|PrintString "SEI SCARSISSIMO" true true "(R=1.000000,G=0.826812,B=0.000000,A=1.000000)" 5.0))))

(event Custom|Start%20Turn
  (TurnManager|PlayerTurn (Variables|Pokemon|GetHUD%20Combat)))

(event Custom|Player%20Attack
  ;[0 0 0 0.5] CUSTOM EVENTS
  (Battle|PlayerAttacking)
  (TurnManager|UpdateUI))

(event Custom|Player%20Switch%20Pokemon
  (params (index :type Integer))
  ;[0 0 0 0.5] CUSTOM EVENTS
  (Development|PrintString "Open Select Pokemon"))

(event Custom|Player%20UseItem
  ;[0 0 0 0.5] CUSTOM EVENTS
)

(event Custom|AddXP
  (bind _asgi_monster_system (CallFunction|GetPkmGameInstance))
  (bind _asgi_monster_system_2 (CallFunction|GetPkmGameInstance))
  ;[0 0 0 0.5] CUSTOM EVENTS
  (Utilities|FlowControl|Delay 1.0)
  (bind _structout (Default|AddXPtoPokemon _asgi_monster_system (Variables|/Game/ThirdPerson/Blueprints/BP_Exploration/GI_MonsterSystem.GI_MonsterSystem_C|GetCurrentPlayerPokemon _asgi_monster_system) 8e+02))
  (Utilities|Array|SetArrayElem (Variables|/Game/ThirdPerson/Blueprints/BP_Exploration/GI_MonsterSystem.GI_MonsterSystem_C|GetPlayerPokemonParty _asgi_monster_system_2) (Variables|/Game/ThirdPerson/Blueprints/BP_Exploration/GI_MonsterSystem.GI_MonsterSystem_C|GetIndexPlayerParty _asgi_monster_system_2) _structout))

(event Custom|EnemyDefeated
  ;[0 0 0 0.5] CUSTOM EVENTS
  (CallFunction|AddXP)
  (Utilities|FlowControl|Delay 1.0)
  (bind (_isbattleended _result _asgi_monster_system) (Battle|IsBattleEnded))
  (if _isbattleended
    (TurnManager|EndBattle)
    (else
      (Default|GetPokemonfromEnemyParty _asgi_monster_system _result)
      (UIHelper|UpdateEnemyUI)
      (CallFunction|TurnFinished))))

(event EventBeginPlay
  (bind _hud_combat (CallFunction|GetCombatHUD))
  ;[0.3389 0.6198 0.5887 0.5] Get Combat HUD
  (Utilities|IsValid (Variables|/Game/Blueprints/Combat/HUD_Combat.HUD_Combat_C|GetWBP%20CombatUI _hud_combat) :!label _label
    (:Is%20Valid
      (Variables|Pokemon|SetHUD%20Combat _hud_combat)
      (DataManager|SetDatafromGameInstance)
      (TurnManager|UpdateUI)
      (CallFunction|StartTurn))
    (:Is%20Not%20Valid
      (Utilities|FlowControl|Delay 0.1)
      (goto _label))))

(fn ConstructionScript)

(fn UpdateUI
  (UIHelper|UpdatePlayerUI)
  (UIHelper|UpdateEnemyUI))

(fn PlayerTurn
  (params (HUD%20Combat :type HUD%20Combat%20Object%20Reference))
  (Development|PrintString "Waiting for player input")
  (Default|ShowActions (Variables|/Game/Blueprints/Combat/HUD_Combat.HUD_Combat_C|GetWBP%20CombatUI HUD%20Combat) "NewEnumerator4"))

(fn EndTurn
  (Development|PrintString "End Turn")
  ;[0.15 0.15 0.15 0.5] IF Should Exit
  (if false
    ;[0.15 0.02833 0.02546 0.5 16] prima di caricare il livello normale salvo i pkm post lotta
    (bind _asgi_monster_system (Utilities|Casting|CastToGI_MonsterSystem (Game|GetGameInstance)))
    (Variables|/Game/ThirdPerson/Blueprints/BP_Exploration/GI_MonsterSystem.GI_MonsterSystem_C|SetPlayerPokemonParty _asgi_monster_system (Variables|Pokemon|GetCurrentPkmList))
    (Game|OpenLevel(byName) (Variables|/Game/ThirdPerson/Blueprints/BP_Exploration/GI_MonsterSystem.GI_MonsterSystem_C|GetMainSceneName _asgi_monster_system))))

(fn SetDatafromGameInstance
  (bind _asgi_monster_system (CallFunction|GetPkmGameInstance))
  (Default|GetPokemonfromPlayerParty _asgi_monster_system)
  (Default|GetPokemonfromEnemyParty _asgi_monster_system))

(fn CalculateDamage
  (params (Attacker :type Pokemon%20Stats%20Structure%20%28by%20ref%29) (Defender :type Pokemon%20Stats%20Structure%20%28by%20ref%29) (Index%20Move :type Integer) (IsDefenderPlayer :type Boolean))
  (bind (_monsterid _monstername _currentlvl _currentexp _neededexp _maxhp _currenthp _atk _def _agility _luck _encounterweight _sprite _model _pokemontype _pokemonmoves) (Utilities|Struct|BreakPokemonStats Attacker))
  (bind _output (Utilities|Array|Get(acopy) _pokemonmoves Index%20Move))
  (bind _damagetype (Variables|/Script/PokeLike.CPP_MoveDataAsset|GetDamageType _output))
  (Variables|Default|SetIsDefenderPlayer IsDefenderPlayer)
  (bind _dmg_base (DamageManager|DmgBase (Math|Conversions|ToFloat(Integer) _atk) (Variables|/Script/PokeLike.CPP_MoveDataAsset|GetDamage _output) (.Def (Utilities|Struct|BreakPokemonStats Defender))))
  ;[0.15 0.15 0.15 0.5] IF CRIT
  (if (< (Math|Random|RandomFloat) (/ _luck 510))
    (bind _output_get (Variables|Pokemon|SetCrit%20Multiplier 1.5))
    (Development|PrintString "CRIT" true true "(R=0.200355,G=1.000000,B=0.241456,A=1.000000)" 1e+01)
    ;[0.15 0.15 0.15 0.5] FINAL CALCULATION CRIT
    (bind _dmgmultiplier (DamageManager|CheckWeaknessResistance _damagetype))
    (Development|PrintString (Utilities|String|Append "CRIT FINAL: " (Utilities|String|ToString(Float) (* (Math|Random|RandomFloatinRange 0.9 1.1) (* (* _dmg_base _output_get) _dmgmultiplier)))) true true "(R=0.027504,G=0.000000,B=1.000000,A=1.000000)" 1e+01)
    (bind _hasdied (DamageManager|FinalDamageCalculation (* (Math|Random|RandomFloatinRange 0.9 1.1) (* (* _dmg_base _output_get) _dmgmultiplier)) Defender))
    (Battle|DecreasePP Attacker Index%20Move)
    (return _hasdied)
    (else
      (bind _output_get_2 (Variables|Pokemon|SetCrit%20Multiplier 1.0))
      (Development|PrintString "NO CRIT" true true "(R=0.531542,G=1.000000,B=0.196943,A=1.000000)" 1e+01)
      ;[0.15 0.15 0.15 0.5] FINAL CALCULATION NO CRIT
      (bind _dmgmultiplier_2 (DamageManager|CheckWeaknessResistance _damagetype))
      (Development|PrintString (Utilities|String|Append "NO CRIT FINAL: " (Utilities|String|ToString(Float) (* (* _dmgmultiplier_2 (* _dmg_base _output_get_2)) (Math|Random|RandomFloatinRange 0.9 1.1)))) true true "(R=1.000000,G=0.022923,B=0.090345,A=1.000000)" 1e+01)
      (bind _hasdied_2 (DamageManager|FinalDamageCalculation (* (* _dmgmultiplier_2 (* _dmg_base _output_get_2)) (Math|Random|RandomFloatinRange 0.9 1.1)) Defender))
      (Battle|DecreasePP Attacker Index%20Move)
      (return _hasdied_2))))

(fn CheckWeaknessResistance
  (params (DamageType :type EMyDamageType%20Enum :default "Option_A"))
  ;[0.15 0.15 0.15 0.5] MyType
  (switch Utilities|FlowControl|Switch|SwitchonEMyDamageType (.PokemonType (Utilities|Struct|BreakPokemonStats (Variables|/Game/ThirdPerson/Blueprints/BP_Exploration/GI_MonsterSystem.GI_MonsterSystem_C|GetCurrentPlayerPokemon (CallFunction|GetPkmGameInstance))))
    (:Option_A
      ;[0.15 0.15 0.15 0.5] POKEMON NORMAL
      (Variables|Pokemon|SetDmg%20Multiplier 1.0)
      (return (Variables|Pokemon|GetDmg%20Multiplier)))
    (:Option_B
      ;[0.15 0.15 0.15 0.5] POKEMON FIRE
      (switch Utilities|FlowControl|Switch|SwitchonEMyDamageType DamageType
        (:Option_A
          (Variables|Pokemon|SetDmg%20Multiplier 1.0))
        (:Option_B
          (Variables|Pokemon|SetDmg%20Multiplier 1.0))
        (:Option_C
          (Variables|Pokemon|SetDmg%20Multiplier 1.5))
        (:Option_D
          (Variables|Pokemon|SetDmg%20Multiplier 0.5)))
      (return (Variables|Pokemon|GetDmg%20Multiplier)))
    (:Option_C
      ;[0.15 0.15 0.15 0.5] POKEMON WATER
      (switch Utilities|FlowControl|Switch|SwitchonEMyDamageType DamageType
        (:Option_A
          (Variables|Pokemon|SetDmg%20Multiplier 1.0))
        (:Option_B
          (Variables|Pokemon|SetDmg%20Multiplier 0.5))
        (:Option_C
          (Variables|Pokemon|SetDmg%20Multiplier 1.0))
        (:Option_D
          (Variables|Pokemon|SetDmg%20Multiplier 1.5)))
      (return (Variables|Pokemon|GetDmg%20Multiplier)))
    (:Option_D
      ;[0.15 0.15 0.15 0.5] POKEMON GRASS
      (switch Utilities|FlowControl|Switch|SwitchonEMyDamageType DamageType
        (:Option_A
          (Variables|Pokemon|SetDmg%20Multiplier 1.0))
        (:Option_B
          (Variables|Pokemon|SetDmg%20Multiplier 1.5))
        (:Option_C
          (Variables|Pokemon|SetDmg%20Multiplier 0.5))
        (:Option_D
          (Variables|Pokemon|SetDmg%20Multiplier 1.0)))
      (return (Variables|Pokemon|GetDmg%20Multiplier)))))

(fn FinalDamageCalculation
  (params (Damage :type Float%20%28double-precision%29) (Defender :type Pokemon%20Stats%20Structure%20%28by%20ref%29))
  (bind _asgi_monster_system (CallFunction|GetPkmGameInstance))
  (bind _structout (Utilities|Struct|SetmembersinPokemonStats Defender (Math|Float|Max(Float) (- (.CurrentHP (Utilities|Struct|BreakPokemonStats Defender)) Damage) 0.0)))
  (Utilities|FlowControl|Sequence
    (:then_0
      ;[0 0 0 0.5] Update Array values
      (if (Variables|Default|GetIsDefenderPlayer)
        (Default|SetPokemonfromPlayerParty _asgi_monster_system _structout)
        (else
          (Default|SetPokemonfromEnemyParty _asgi_monster_system _structout))))
    (:then_1
      (return (<= (.CurrentHP (Utilities|Struct|BreakPokemonStats Defender)) 0.0)))))

(fn DmgBase
  (params (Atk :type Float%20%28double-precision%29) (Move%20Multiplier :type Float%20%28double-precision%29) (OpponentDef :type Integer))
  (return (|(((pow(Atk,ExpAtk))/((pow(Def,ExpDef))+1))*Mult) Atk (Math|Conversions|ToFloat(Integer) OpponentDef) Move%20Multiplier 1.2 0.9)))

(fn CheckFirstAttacker
  (bind _asgi_monster_system (CallFunction|GetPkmGameInstance))
  (return (>= (.Agility (Utilities|Struct|BreakPokemonStats (Variables|/Game/ThirdPerson/Blueprints/BP_Exploration/GI_MonsterSystem.GI_MonsterSystem_C|GetCurrentPlayerPokemon _asgi_monster_system))) (.Agility (Utilities|Struct|BreakPokemonStats (Variables|/Game/ThirdPerson/Blueprints/BP_Exploration/GI_MonsterSystem.GI_MonsterSystem_C|GetCurrentEnemyPokemon _asgi_monster_system))))))

(fn PlayerAttacking
  (bind _asgi_monster_system (CallFunction|GetPkmGameInstance))
  (bind _hasdied (DamageManager|CalculateDamage (Variables|/Game/ThirdPerson/Blueprints/BP_Exploration/GI_MonsterSystem.GI_MonsterSystem_C|GetCurrentPlayerPokemon _asgi_monster_system) (Variables|/Game/ThirdPerson/Blueprints/BP_Exploration/GI_MonsterSystem.GI_MonsterSystem_C|GetCurrentEnemyPokemon _asgi_monster_system) (Variables|Default|GetPlayerMoveIndex) false))
  (Variables|Default|SetIsEnemyDead _hasdied)
  (return))

(fn EnemyAttacking
  (bind _asgi_monster_system (CallFunction|GetPkmGameInstance))
  (bind _currentenemypokemon (Variables|/Game/ThirdPerson/Blueprints/BP_Exploration/GI_MonsterSystem.GI_MonsterSystem_C|GetCurrentEnemyPokemon _asgi_monster_system))
  (bind _hasdied (DamageManager|CalculateDamage _currentenemypokemon (Variables|/Game/ThirdPerson/Blueprints/BP_Exploration/GI_MonsterSystem.GI_MonsterSystem_C|GetCurrentPlayerPokemon _asgi_monster_system) (CallFunction|GetRandomMoveIndex _currentenemypokemon) true))
  (Variables|Default|SetIsPlayerDead _hasdied)
  (return))

(fn EndBattle
  (bind _returnvalue (Game|GetPlayerController 0))
  (Game|OpenLevel(byObjectReference) "/Game/Levels/LVL_Encounter_Test.LVL_Encounter_Test")
  (Input|SetInputModeGameOnly _returnvalue false)
  (Variables|/Script/Engine.PlayerController|SetbShowMouseCursor _returnvalue false))

(fn UpdatePlayerUI
  (Default|UpdateMyPkmStats (Variables|/Game/Blueprints/Combat/HUD_Combat.HUD_Combat_C|GetWBP%20CombatUI (CallFunction|GetCombatHUD)) (Variables|/Game/ThirdPerson/Blueprints/BP_Exploration/GI_MonsterSystem.GI_MonsterSystem_C|GetCurrentPlayerPokemon (CallFunction|GetPkmGameInstance))))

(fn UpdateEnemyUI
  (Default|UpdateOppoPkmStats (Variables|/Game/Blueprints/Combat/HUD_Combat.HUD_Combat_C|GetWBP%20CombatUI (CallFunction|GetCombatHUD)) (Variables|/Game/ThirdPerson/Blueprints/BP_Exploration/GI_MonsterSystem.GI_MonsterSystem_C|GetCurrentEnemyPokemon (CallFunction|GetPkmGameInstance))))

(fn IsBattleEnded
  (bind _asgi_monster_system (CallFunction|GetPkmGameInstance))
  (bind _result (Math|Integer|IncrementInt (Variables|/Game/ThirdPerson/Blueprints/BP_Exploration/GI_MonsterSystem.GI_MonsterSystem_C|GetIndexEnemyParty _asgi_monster_system))
    (:%20%20
      (return (>= _result (Utilities|Array|Length (Variables|/Game/ThirdPerson/Blueprints/BP_Exploration/GI_MonsterSystem.GI_MonsterSystem_C|GetEnemyPokemonParty (CallFunction|GetPkmGameInstance)))) _result _asgi_monster_system))))

(fn DecreasePP
  (params (PokemonStats :type Pokemon%20Stats%20Structure%20%28by%20ref%29) (Index :type Integer))
  (bind _currentpp (CallFunction|GetCurrentMovePP PokemonStats Index))
  (CallFunction|SetCurrentMovePP PokemonStats Index (- _currentpp 1)))

(fn GetRandomMoveIndex
  (params (Pokemon :type Pokemon%20Stats%20Structure))
  (bind _output_get (LocalVariables|SetLocal_MoveSet (.PokemonMoves (Utilities|Struct|BreakPokemonStats Pokemon))))
  (bind _result (Math|Integer|DecrementInt (Utilities|Array|Length _output_get))
    (:%20%20
      (return (Math|Random|RandomInteger _result)))))

(fn GetCurrentMovePP
  (params (Pokemon :type Pokemon%20Stats%20Structure%20%28by%20ref%29) (MoveIndex :type Integer))
  (return (Utilities|Struct|BreakPkmMove (Utilities|Array|Get(acopy) (.CurrentMoves (Utilities|Struct|BreakPokemonStats Pokemon)) MoveIndex))))

(fn SetCurrentMovePP
  (params (Pokemon :type Pokemon%20Stats%20Structure%20%28by%20ref%29) (MoveIndex :type Integer) (CurrentPP :type Integer))
  (Utilities|Struct|SetmembersinPkmMove (Utilities|Array|Get(acopy) (.CurrentMoves (Utilities|Struct|BreakPokemonStats Pokemon)) MoveIndex) CurrentPP))