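; HUD for combat that shows the combat UI and relays the player's confirmed action to the combat game mode.
; On BeginPlay it creates the WBP_CombatUI widget, switches input to UI-only with a visible cursor, and binds to its own OnActionConfirmed dispatcher.
; ConfirmAction fires that dispatcher, whose handler disables the widget's actions and calls OnSelectedPkmAction on the game mode.
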(event Custom|OnActionConfirmed_Event
  (Default|DisableActions (Variables|Default|GetWBP%20CombatUI))
  (Default|OnSelectedPkmAction (CallFunction|GetCombatGameMode)))

(event EventBeginPlay
  (bind _returnvalue (Game|GetPlayerController 0))
  (Utilities|FlowControl|Sequence
    (:then_0
      (bind _returnvalue_2 (UserInterface|CreateWidget "/Game/Blueprints/UI/Combat/WBP_CombatUI.WBP_CombatUI_C" _returnvalue))
      (bind _output_get (Variables|Default|SetWBP%20CombatUI _returnvalue_2))
      (UserInterface|Viewport|AddtoViewport _output_get 0)
      (Input|SetInputModeUIOnly _returnvalue _output_get "DoNotLock" false)
      (Variables|/Script/Engine.PlayerController|SetbShowMouseCursor _returnvalue true))
    (:then_1
      (EventDispatchers|BindEventtoOnActionConfirmed (delegate Custom|OnActionConfirmed_Event)))))

(fn ConstructionScript)

(fn ConfirmAction
  (Default|CallOnActionConfirmed))