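; BFL_Poke is a function library of shortcut getters for the core framework objects of a monster combat game.
; It returns the combat HUD, world HUD, monster-system game instance and combat game mode, each cast to its project class.
; Both HUD getters read from player controller 0 and print an error on a failed cast, while the other two getters fail silently.
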(fn GetCombatHUD
  (bind _ashud_combat (Utilities|Casting|CastToHUD_Combat (HUD|GetHUD (Game|GetPlayerController 0)))
    (:then
      (return _ashud_combat))
    (:CastFailed
      (Development|PrintString 0 "CAST FAILED"))))

(fn GetPkmGameInstance
  (bind _asgi_monster_system (Utilities|Casting|CastToGI_MonsterSystem (Game|GetGameInstance)))
  (return _asgi_monster_system))

(fn GetCombatGameMode
  (bind _asbp_combat_game_mode (Utilities|Casting|CastToBP_CombatGameMode (Game|GetGameMode)))
  (return _asbp_combat_game_mode))

(fn GetWorldHUD
  (bind _ashud_world (Utilities|Casting|CastToHUD_World (HUD|GetHUD (Game|GetPlayerController 0)))
    (:then
      (return _ashud_world))
    (:CastFailed
      (Development|PrintString 0 "CAST FAILED"))))