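; BP_Warp is a warp trigger actor that teleports the third-person player character to a target actor's location.
; On overlap it checks the other actor is the player character, deactivates its movement and fades the camera out.
; After a short delay it moves the player to the target with an X offset, keeping rotation, then fades back in and reactivates movement.
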(event EventBeginPlay)

(event Collision|EventActorBeginOverlap
  (params (OtherActor :type Actor%20Object%20Reference))
  (bind _teleport_target (Variables|Teleport|GetTeleport_Target))
  (bind _returnvalue (Transformation|GetActorLocation _teleport_target))
  (bind _returnvalue_2 (Actor|GetActorOfClass "/Game/ThirdPerson/Blueprints/BP_ThirdPersonCharacter.BP_ThirdPersonCharacter_C"))
  (if (== _returnvalue_2 OtherActor)
    (Development|PrintString "IS_Player")
    (bind _output_get (Variables|Teleport|SetPlayer_Actor _returnvalue_2))
    (bind _asbp_third_person_character (Utilities|Casting|CastToBP_ThirdPersonCharacter _output_get))
    (Components|Activation|Deactivate (Variables|/Script/Engine.Character|GetCharacterMovement _asbp_third_person_character))
    (Development|PrintString "Teleport")
    (CameraFades|StartCameraFade :self (Variables|/Script/Engine.PlayerController|GetPlayerCameraManager (Game|GetPlayerController 0)) :ToAlpha 1.0 :Duration 0.5 :bHoldWhenFinished true)
    (Utilities|FlowControl|Delay 1.0)
    (Transformation|SetActorLocationAndRotation _output_get (Math|Vector|MakeVector (+ (Variables|Teleport|GetOffset_Position) (.x _returnvalue)) (.y _returnvalue) (.z _returnvalue)) (Transformation|GetActorRotation _output_get) false true)
    (CameraFades|StartCameraFade :self (Variables|/Script/Engine.PlayerController|GetPlayerCameraManager (Game|GetPlayerController 0)) :FromAlpha 1.0 :Duration 0.5)
    (bind _asbp_third_person_character_2 (Utilities|Casting|CastToBP_ThirdPersonCharacter (Variables|Teleport|GetPlayer_Actor)))
    (Components|Activation|Activate (Variables|/Script/Engine.Character|GetCharacterMovement _asbp_third_person_character_2) false)
    (else
      (Development|PrintString "IS_Not_player"))))

(event EventTick
  (params (DeltaSeconds :type Float%20%28single-precision%29))
  (Variables|Default|SetDelta%20Seconds DeltaSeconds))

(fn ConstructionScript)